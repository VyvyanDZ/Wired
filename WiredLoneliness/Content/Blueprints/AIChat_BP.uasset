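; AIChat_BP is a chatbot terminal actor that lets the player type messages on a Terminal widget and shows bot replies.
; Overlap enables input, and an AnyKey handler appends key display names to the input text, filtering out mouse, arrow, Space, Backspace and Enter keys.
; Enter passes the text to GetUserInput, then fetches GetBotResponse, both defined outside these graphs.
; User and AI messages each fill three-line scrolling histories.
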(event `self.ReceiveActorBeginOverlap`
  (params (OtherActor :type "Actor Object Reference"))
  (bind _returnvalue (`GameplayStatics.GetPlayerController` 0))
  (`self.EnableInput` (`GameplayStatics.GetPlayerController` 0))
  (bind _asterminal (cast `/Game/Blueprints/Terminal` (`WidgetComponent.GetUserWidgetObject` (`self.Terminal`))))
  (if (or (`PlayerController.IsInputKeyDown` _returnvalue "LeftMouseButton") (`PlayerController.IsInputKeyDown` _returnvalue "RightMouseButton") (`PlayerController.IsInputKeyDown` _returnvalue "SpaceBar") (`PlayerController.IsInputKeyDown` _returnvalue "BackSpace") (`PlayerController.IsInputKeyDown` _returnvalue "Enter") (`PlayerController.IsInputKeyDown` _returnvalue "Up") (`PlayerController.IsInputKeyDown` _returnvalue "Down") (`PlayerController.IsInputKeyDown` _returnvalue "Right") (`PlayerController.IsInputKeyDown` _returnvalue "Left")) :!label _label
    (if (`PlayerController.IsInputKeyDown` (`GameplayStatics.GetPlayerController` 0) "Enter")
      (bind _userinput (`/Game/Blueprints/Terminal.UserInput` _asterminal))
      (bind _returnvalue_2 (`TextBlock.GetText` _userinput))
      (bind _returnvalue_3 (`self.getUserInput` (`KismetTextLibrary.Conv_TextToString` _returnvalue_2)))
      (bind _useroutput1 (`/Game/Blueprints/Terminal.UserOutput1` _asterminal))
      (if (`KismetTextLibrary.TextIsEmpty` (`TextBlock.GetText` _useroutput1))
        (bind _returnvalue_4 (`KismetTextLibrary.Conv_StringToText` _returnvalue_3))
        (`TextBlock.SetText` _useroutput1 _returnvalue_4)
        (else
          (bind _useroutput2 (`/Game/Blueprints/Terminal.UserOutput2` _asterminal))
          (bind _returnvalue_5 (`TextBlock.GetText` _useroutput2))
          (if (`KismetTextLibrary.TextIsEmpty` _returnvalue_5)
            (`TextBlock.SetText` _useroutput2 _returnvalue_4)
            (else
              (bind _useroutput3 (`/Game/Blueprints/Terminal.UserOutput3` _asterminal))
              (bind _returnvalue_6 (`TextBlock.GetText` _useroutput3))
              (if (`KismetTextLibrary.TextIsEmpty` _returnvalue_6)
                (`TextBlock.SetText` _useroutput3 _returnvalue_4)
                (else
                  (`TextBlock.SetText` _useroutput1 _returnvalue_5)
                  (`TextBlock.SetText` _useroutput2 _returnvalue_6)
                  (`TextBlock.SetText` _useroutput3 _returnvalue_4)))))))
      (`TextBlock.SetText` _userinput "")
      (bind _returnvalue_7 (`self.getBotResponse`))
      (bind _aioutput1 (`/Game/Blueprints/Terminal.AIOutput1` _asterminal))
      (if (`KismetTextLibrary.TextIsEmpty` (`TextBlock.GetText` _aioutput1))
        (bind _returnvalue_8 (`KismetTextLibrary.Conv_StringToText` _returnvalue_7))
        (`TextBlock.SetText` _aioutput1 _returnvalue_8)
        (else
          (bind _aioutput2 (`/Game/Blueprints/Terminal.AIOutput2` _asterminal))
          (bind _returnvalue_9 (`TextBlock.GetText` _aioutput2))
          (if (`KismetTextLibrary.TextIsEmpty` _returnvalue_9)
            (`TextBlock.SetText` _aioutput2 _returnvalue_8)
            (else
              (bind _aioutput3 (`/Game/Blueprints/Terminal.AIOutput3` _asterminal))
              (bind _returnvalue_10 (`TextBlock.GetText` _aioutput3))
              (if (`KismetTextLibrary.TextIsEmpty` _returnvalue_10)
                (`TextBlock.SetText` _aioutput3 _returnvalue_8)
                (else
                  (`TextBlock.SetText` _aioutput1 _returnvalue_9)
                  (`TextBlock.SetText` _aioutput2 _returnvalue_10)
                  (`TextBlock.SetText` _aioutput3 _returnvalue_8))))))))
    (else
      (`TextBlock.SetText` _userinput (`KismetTextLibrary.Conv_StringToText` (`KismetStringLibrary.Concat_StrStr` (`KismetTextLibrary.Conv_TextToString` _returnvalue_2) (`KismetTextLibrary.Conv_TextToString` (`KismetInputLibrary.Key_GetDisplayName` (stale `Key|AnyKey` Key)))))))))

(event `Key|AnyKey`
  (params (Key :type "Key Structure" :default "AnyKey"))
  (:`Pressed`
    (goto _label)))

(fn `UserConstructionScript`)