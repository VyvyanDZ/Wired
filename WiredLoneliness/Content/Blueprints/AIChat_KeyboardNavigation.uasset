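; Interactable in-world AI chat station that lets the player operate its Menu, Terminal and CommandLine widgets by keyboard.
; Overlap shows the ClickE prompt and enables input; pressing E switches the view target to the actor and activates the menu.
; It links the widgets to each other and itself, then forwards any key press to Terminal chat if active, otherwise to an active CommandLine.
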(event `self.ReceiveActorBeginOverlap`
  (params (OtherActor :type "Actor Object Reference"))
  (bind _returnvalue (`GameplayStatics.GetPlayerController` 0))
  (`SceneComponent.SetVisibility` (`self.Click e`) true false)
  (bind _asmenu (cast `/Game/Blueprints/menu` (`WidgetComponent.GetUserWidgetObject` (`self.Menu`))))
  (bind _output_get (set `/Game/Blueprints/menu.isActive` true _asmenu))
  (`self.EnableInput` _returnvalue)
  (if (and _output_get (`PlayerController.IsInputKeyDown` _returnvalue (stale `Key|E` Key))) :!label _label
    (`SceneComponent.SetVisibility` (`self.Click e`) false false)
    (`PlayerController.SetViewTargetWithBlend` (`GameplayStatics.GetPlayerController` 0) self 0.0 "VTBlend_Linear" 0.0 true)
    (`/Game/Blueprints/menu.Menu activated` _asmenu)
    (bind _asterminal (cast `/Game/Blueprints/Terminal` (`WidgetComponent.GetUserWidgetObject` (`self.Terminal`))))
    (`/Game/Blueprints/menu.SetTerminal` _asmenu _asterminal)
    (`/Game/Blueprints/Terminal.SetAichat` _asterminal self)
    (if (`/Game/Blueprints/Terminal.isActive` _asterminal) :!label _label_2
      (`/Game/Blueprints/Terminal.Chat` (`/Game/Blueprints/menu.Terminal` _asmenu) (stale `Key|AnyKey` Key))
      (else
        (bind _ascommand_line (cast `/Game/Blueprints/CommandLine` (`WidgetComponent.GetUserWidgetObject` (`self.CommandLine`))))
        (`/Game/Blueprints/menu.SetCommandLine` _asmenu _ascommand_line)
        (`/Game/Blueprints/CommandLine.SetAichat` _ascommand_line self)
        (if (`/Game/Blueprints/CommandLine.isActive` _ascommand_line)
          (`/Game/Blueprints/CommandLine.Command` _ascommand_line (stale `Key|AnyKey` Key)))))))

(event `Key|AnyKey`
  (params (Key :type "Key Structure" :default "AnyKey"))
  (:`Pressed`
    (goto _label_2)))

(event `Key|E`
  (params (Key :type "Key Structure" :default "AnyKey"))
  (:`Pressed`
    (goto _label)))

(fn `UserConstructionScript`)