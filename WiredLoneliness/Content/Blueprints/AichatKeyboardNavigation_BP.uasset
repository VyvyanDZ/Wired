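; Interactive actor that lets the player operate an in-world command-line terminal by keyboard, apparently for an AI chat.
; On overlap it gets the cmd widget from its CMD component, shows the ClickE prompt and enables player input.
; Pressing E while inactive hides the prompt, switches the view to the actor, activates the command line and registers itself with it.
; While active, an AnyKey handler forwards pressed keys to the widget.
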(event `self.ReceiveActorBeginOverlap`
  (params (OtherActor :type "Actor Object Reference"))
  (bind _returnvalue (`GameplayStatics.GetPlayerController` 0))
  (bind _ascmd (cast `/Game/Blueprints/cmd` (`WidgetComponent.GetUserWidgetObject` (`self.CMD`))))
  (`SceneComponent.SetVisibility` (`self.Click e`) true false)
  (`self.EnableInput` _returnvalue)
  (bind _isactive (`/Game/Blueprints/cmd.isActive` _ascmd))
  (if (and (not _isactive) (`PlayerController.IsInputKeyDown` _returnvalue "E")) :!label _label
    (`SceneComponent.SetVisibility` (`self.Click e`) false false)
    (`PlayerController.SetViewTargetWithBlend` _returnvalue self 0.0 "VTBlend_Linear" 0.0 true)
    (`/Game/Blueprints/cmd.commandLine activated` _ascmd)
    (`/Game/Blueprints/cmd.SetAichat` _ascmd self)
    (elif (and (`PlayerController.IsInputKeyDown` (`GameplayStatics.GetPlayerController` 0) (stale `Key|AnyKey` Key)) _isactive)
      (`/Game/Blueprints/cmd.Command` _ascmd (stale `Key|AnyKey` Key)))))

(event `Key|AnyKey`
  (params (Key :type "Key Structure" :default "AnyKey"))
  (:`Pressed`
    (goto _label)))

(fn `UserConstructionScript`)